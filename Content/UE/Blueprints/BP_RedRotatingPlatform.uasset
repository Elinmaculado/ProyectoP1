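; Red rotating platform that spins on its pitch axis and slows down temporarily when it takes red damage.
; Tick applies a local pitch rotation scaled by delta time and RotationSpeed while the IsRotationg flag is set.
; TakeRedDamage drops the speed to a slow value, waits through a short Delay, then sets a hard-coded fast speed rather than restoring the previous one.
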(event EventTick
  (params (DeltaSeconds :type Float%20%28single-precision%29))
  (if (Variables|Default|GetIsRotationg)
    (Transformation|AddActorLocalRotation (Math|Rotator|MakeRotator 0.0 (* DeltaSeconds (Variables|Default|GetRotationSpeed)) 0.0) false false)))

(event EventTakeRedDamage
  (Variables|Default|SetRotationSpeed -5.0)
  (Utilities|FlowControl|Delay 2.0)
  (Variables|Default|SetRotationSpeed -5e+01))

(fn ConstructionScript
  (|CallParentFunction))