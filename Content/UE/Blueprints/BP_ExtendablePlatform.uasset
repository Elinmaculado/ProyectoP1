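; BP_ExtendablePlatform is a platform that lengthens when it takes red damage and shortens when it takes blue damage.
; Each hit changes the actor's Y scale by one step and shifts it along world Y by a fixed offset, apparently to anchor one end.
; The scale stored at BeginPlay gates retraction, while extension has no upper limit.
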(event EventTakeBlueDamage
  (if (< (.y (Variables|Default|GetInitialScale)) (.y (Transformation|GetActorScale3D)))
    (Transformation|SetActorScale3D (- (Transformation|GetActorScale3D) "0.000000,1.000000,0.000000"))
    (Transformation|SetActorLocation (+ (Transformation|GetActorLocation) "0.000000,90.000000,0.000000") false false)))

(event EventBeginPlay
  ;[0.15 0.15 0.15 0.5] Obtenemos tamaño inicial
  (Variables|Default|SetInitialScale (Transformation|GetActorScale3D)))

(event EventTakeRedDamage
  (Transformation|SetActorScale3D (+ (Transformation|GetActorScale3D) "0.000000,1.000000,0.000000"))
  (Transformation|SetActorLocation (- (Transformation|GetActorLocation) "0.000000,90.000000,0.000000") false false))

(fn ConstructionScript)