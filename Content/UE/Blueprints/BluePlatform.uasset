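; BluePlatform is an actor that temporarily turns from a cube into a plane when it takes blue damage.
; It starts with the Plane hidden and non-colliding, and TakeBlueDamage swaps visibility and collision from the Cube to the Plane.
; After a two-second delay, ResetShape restores the Cube and hides the Plane again.
; A disconnected chain holds an alternative mesh-swap version that never runs.
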(event Custom|Reset%20shape
  (Rendering|SetVisibility (Variables|Default|GetPlane) false false)
  (Collision|SetCollisionEnabled (Variables|Default|GetPlane) "NoCollision")
  (Rendering|SetVisibility (Variables|Default|GetCube) true false)
  (Collision|SetCollisionEnabled (Variables|Default|GetCube) "QueryAndPhysics"))

(event EventTakeBlueDamage
  (Rendering|SetVisibility (Variables|Default|GetPlane) true false)
  (Collision|SetCollisionEnabled (Variables|Default|GetPlane) "QueryAndPhysics")
  (Rendering|SetVisibility (Variables|Default|GetCube) false false)
  (Collision|SetCollisionEnabled (Variables|Default|GetCube) "NoCollision")
  (Utilities|FlowControl|Delay 2.0)
  (CallFunction|ResetShape))

(event EventBeginPlay
  (Rendering|SetVisibility (Variables|Default|GetPlane) false false)
  (Collision|SetCollisionEnabled (Variables|Default|GetPlane) "NoCollision"))

(fn ConstructionScript
  (|CallParentFunction))